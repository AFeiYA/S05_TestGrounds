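; BP_Tile is a tile of infinite terrain that scatters a random handful of BP_Container actors on itself at BeginPlay.
; Player overlap with BarriorTrigger turns the barrier green and passable; leaving restores red and solid.
; Player overlap with DestoryTrigger destroys the tile and asks InfiniteTerrainGameMode to spawn another.
; GetAttachedLocationEast exposes the AttachLocationEast world transform as an attachment point.
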(event OnComponentBeginOverlap(BarriorTrigger)
  (params (OverlappedComponent :type Primitive%20Component%20Object%20Reference) (OtherActor :type Actor%20Object%20Reference) (OtherComp :type Primitive%20Component%20Object%20Reference) (OtherBodyIndex :type Integer) (bFromSweep :type Boolean) (SweepResult :type Hit%20Result%20Structure%20%28by%20ref%29))
  (Utilities|IsPlayer OtherActor)
  (Collision|SetCollisionEnabled (Variables|Default|GetBarrior) "NoCollision")
  (Rendering|Material|SetMaterial (Variables|Default|GetBarrior) 0 "/Game/Static/Geometry/Meshes/M_Barrior_Inst_Green.M_Barrior_Inst_Green"))

(event OnComponentEndOverlap(BarriorTrigger)
  (params (OverlappedComponent :type Primitive%20Component%20Object%20Reference) (OtherActor :type Actor%20Object%20Reference) (OtherComp :type Primitive%20Component%20Object%20Reference) (OtherBodyIndex :type Integer))
  (Utilities|IsPlayer OtherActor)
  (Collision|SetCollisionEnabled (Variables|Default|GetBarrior) "QueryAndPhysics")
  (Rendering|Material|SetMaterial (Variables|Default|GetBarrior) 0 "/Game/Static/Geometry/Meshes/M_Barrior_Inst_Red.M_Barrior_Inst_Red"))

(event OnComponentBeginOverlap(DestoryTrigger)
  (params (OverlappedComponent :type Primitive%20Component%20Object%20Reference) (OtherActor :type Actor%20Object%20Reference) (OtherComp :type Primitive%20Component%20Object%20Reference) (OtherBodyIndex :type Integer) (bFromSweep :type Boolean) (SweepResult :type Hit%20Result%20Structure%20%28by%20ref%29))
  (Utilities|IsPlayer OtherActor)
  (Actor|DestroyActor)
  (bind _asinfinite_terrain_game_mode (Utilities|Casting|CastToInfiniteTerrainGameMode (Game|GetGameMode)))
  (Default|SpawnTile _asinfinite_terrain_game_mode))

(event EventBeginPlay
  (Rendering|Material|SetMaterial (Variables|Default|GetBarrior) 0 "/Game/Static/Geometry/Meshes/M_Barrior_Inst_Red.M_Barrior_Inst_Red")
  (Class|Tile|PlaceActors "/Game/Dynamic/Props/BP_Container.BP_Container_C" 1 5))

(event Collision|EventActorBeginOverlap
  (params (OtherActor :type Actor%20Object%20Reference)))

(event EventTick
  (params (DeltaSeconds :type Float%20%28single-precision%29)))

(fn ConstructionScript)

(fn GetAttachedLocationEast
  (return (Transformation|GetWorldTransform (Variables|Default|GetAttachLocationEast))))